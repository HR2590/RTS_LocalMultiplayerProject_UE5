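; RTS game mode that sets up each joining player with an index, main UI, identity and world cursor.
; On player start, it picks a name and color from the PlayerInfo map by controller count, spawns an owned BP_Cursor and passes the info to PS_Rts.
; Cursors are mapped by controller for repositioning, and getters lazily cache single controller and game state references.
; UpdateCursors and UpdatePlayersInfoHUD are empty stubs.
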(event `self.HandleStartingNewPlayer`
  (params (NewPlayer :type "PlayerController Object Reference"))
  (bind (_name _color) (`self.GetPlayerBasicInfo`))
  ;[1 0 0] NewPlayerStart
  (bind _aspc_rts (cast `/Game/Blueprint/Core/Gameflow/Playercontrollers/PC_Rts` NewPlayer)
    (:`then`
      (`/Game/Blueprint/Core/Gameflow/Playercontrollers/PC_Rts.SetPlayerIndex` _aspc_rts (- (`KismetArrayLibrary.Array_Length` (`GameStateBase.PlayerArray` (`GameplayStatics.GetGameState`))) 1))
      (`/Game/Blueprint/Core/Gameflow/Playercontrollers/PC_Rts.LoadMainUI` _aspc_rts)
      (`self.CreateCursor` NewPlayer (`GameplayStatics.GetNumPlayerControllers`))
      (bind _asps_rts (cast `/Game/Blueprint/Core/Gameflow/PlayerStates/PS_Rts` (`Controller.PlayerState` NewPlayer)))
      (`/Game/Blueprint/Core/Gameflow/PlayerStates/PS_Rts.AddPlayersInfo` _asps_rts _name _color (`GameplayStatics.GetNumPlayerControllers`))
      (`parent.HandleStartingNewPlayer` NewPlayer))
    (:`CastFailed`
      (`KismetSystemLibrary.PrintString` "Cast Failed"))))

(fn `CreateCursor`
  (params (PC :type "PlayerController Object Reference") (PlayerIndex :type Integer))
  (bind _returnvalue (- PlayerIndex 1))
  ;[1 0 0] CreateNewCursor
  (bind _keys (`BlueprintMapLibrary.Map_Keys` (`self.PlayerInfo`)))
  (bind _values (`BlueprintMapLibrary.Map_Values` (`self.PlayerInfo`)))
  (bind _returnvalue_2 (`|SpawnActorFromClass` "/Game/Blueprint/Core/Interactables/ActorCursor/BP_Cursor.BP_Cursor_C" (`KismetMathLibrary.MakeTransform` (0.0 0.0 0.0)) "Undefined" "MultiplyWithRoot" PC (`|GetArrayItem` _values _returnvalue) (`|GetArrayItem` _keys _returnvalue) null))
  (`BlueprintMapLibrary.Map_Add` (`self.Cursors`) PC _returnvalue_2))

(fn `GetGSRef`
  (returns (GSRef :type "/Game/Blueprint/Core/Gameflow/GameStates/GS_Rts Object Reference"))
  (`self.GSRef`
    (:`then`
      _)
    (:`else`
      (bind _asgs_rts (cast `/Game/Blueprint/Core/Gameflow/GameStates/GS_Rts` (`GameplayStatics.GetGameState`)))
      (set `self.GSRef` _asgs_rts)))
  (return (`self.GSRef`)))

(fn `GetPCRef`
  (params (PlayerIndex :type Integer))
  (returns (PCRts :type "/Game/Blueprint/Core/Gameflow/Playercontrollers/PC_Rts Object Reference"))
  (`self.PCRts`
    (:`then`
      _)
    (:`else`
      (bind _aspc_rts (cast `/Game/Blueprint/Core/Gameflow/Playercontrollers/PC_Rts` (`GameplayStatics.GetPlayerController` PlayerIndex)))
      (set `self.PCRts` _aspc_rts)))
  (return (`self.PCRts`)))

(fn `GetPlayerBasicInfo`
  (returns (Name :type "Name (by ref)") (Color :type "Color Structure (by ref)"))
  (bind _returnvalue (- (`GameplayStatics.GetNumPlayerControllers`) 1))
  (bind _keys (`BlueprintMapLibrary.Map_Keys` (`self.PlayerInfo`)))
  (bind _values (`BlueprintMapLibrary.Map_Values` (`self.PlayerInfo`)))
  (return (`|GetArrayItem` _keys _returnvalue) (`|GetArrayItem` _values _returnvalue)))

(fn `GetPlayerColor`
  (params (Index :type Integer))
  (returns (PlayerColor :type "Color Structure"))
  (bind _values (`BlueprintMapLibrary.Map_Values` (`self.PlayerInfo`)))
  (return (`|GetArrayItem` _values Index)))

(fn `SetCursorPosition`
  (params (PC :type "PlayerController Object Reference") (Position :type "Vector Structure"))
  (bind (_value _returnvalue) (`BlueprintMapLibrary.Map_Find` (`self.Cursors`) PC))
  (if _returnvalue
    (`self.K2_SetActorLocation` _value Position false false)))

(fn `UpdateCursors`)

(fn `UpdatePlayersInfoHUD`)

(fn `UserConstructionScript`)