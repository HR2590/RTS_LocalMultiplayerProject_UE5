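; RTS player pawn that drives the camera, object selection, building placement, unit orders and map marks.
; Left-click traces place buildings, set rally points, or select actors with player-colored decals shown through multicast, updating the HUD through PC_Rts.
; Right mouse pans and orders the selected unit to move, gather or construct, while middle-click opens map marking.
; Zoom plays or reverses a timeline that blends camera height and pitch from curve endpoints.
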(event `EnhancedInput|/Game/Blueprint/Core/Input/IA_Movement`
  (params (ActionValue :type "Vector2D Structure") (ElapsedSeconds :type "Float (double-precision)") (TriggeredSeconds :type "Float (double-precision)") (InputAction :type "InputAction Object Reference" :default "/Game/Blueprint/Core/Input/IA_Movement.IA_Movement"))
  (:`Triggered`
    (`PawnMovementComponent.AddInputVector` (`self.FloatingPawnMovement`) (`KismetMathLibrary.Conv_Vector2DToVector` ActionValue) false)))

(event `OnSpawnBuilding`
  (params (Position :type "Vector Structure"))
  (bind _previewbuilding (`self.PreviewBuilding`))
  ;[1 0 0] spawnBuilding
  (if (`KismetSystemLibrary.IsValid` _previewbuilding)
    (if (`/Game/Blueprint/Core/Interactables/BaseActorsRTS/PreviewBuilding.Can Place` _previewbuilding)
      (`|SpawnActorFromClass` "/Game/Blueprint/Core/Interactables/BaseActorsRTS/BaseBuilding.BaseBuilding_C" (`KismetMathLibrary.MakeTransform` Position) "Undefined" "MultiplyWithRoot" null (`/Game/Blueprint/Core/Interactables/BaseActorsRTS/PreviewBuilding.ClassTag` (`self.PreviewBuilding`)) (`self.GetPSRef`) true null)
      (`self.K2_DestroyActor` (`self.PreviewBuilding`)))))

(event `EnhancedInput|/Game/Blueprint/Core/Input/IA_Left`
  (params (ActionValue :type Boolean) (ElapsedSeconds :type "Float (double-precision)") (TriggeredSeconds :type "Float (double-precision)") (InputAction :type "InputAction Object Reference" :default "/Game/Blueprint/Core/Input/IA_Left.IA_Left"))
  (bind (_outhit _returnvalue) (`self.GetMousePosition` "TraceTypeQuery3"))
  (bind _lasactorselected (`self.LasActorSelected`))
  (bind (_bblockinghit _binitialoverlap _time _distance _location _impactpoint _normal _impactnormal _physmat _hitactor _hitcomponent) (`GameplayStatics.BreakHitResult` _outhit))
  (bind _returnvalue_2 (`self.GetComponentByClass` _lasactorselected "/Game/Blueprint/Core/Interactables/Components/AC_BuildingInfo.AC_BuildingInfo_C"))
  (bind _returnvalue_3 (`PrimitiveComponent.GetCollisionObjectType` _hitcomponent))
  (bind _returnvalue_4 (`|EnumEquality` _returnvalue_3 "ECC_GameTraceChannel7"))
  ;[0 0.1646 1] Left click Select Object
  (:`Started`
    (if _bblockinghit
      (if (or _returnvalue_4 (`|EnumEquality` _returnvalue_3 "ECC_GameTraceChannel8"))
        (`/Game/Blueprint/Core/Gameflow/Playercontrollers/PC_Rts.spawnBuilding` (`self.GetPCRef`) _location)
        (if (and _returnvalue_4 (`KismetSystemLibrary.IsValid` _lasactorselected))
          (if (`KismetSystemLibrary.IsValid` _returnvalue_2)
            (bind _output_get (set `/Game/Blueprint/Core/Interactables/Components/AC_BaseInfo.RallyPoint` _location _returnvalue_2))
            (`/Game/Blueprint/Core/Gameflow/Playercontrollers/PC_Rts.SaveRallyPoint` (`self.GetPCRef`) _output_get)))
        (elif _returnvalue
          (`self.DeselectOnServer`)
          (`self.AddDecalOnServer` _hitactor)
          (bind _output_get_2 (set `self.LasActorSelected` _hitactor))
          (`self.GetObjectInfo` _output_get_2)
          (else
            (`self.DeselectOnServer`))))
      (else
        (`self.DeselectOnServer`)))))

(event `GetObjectInfo`
  (params (InActor :type "Actor Object Reference"))
  (bind _returnvalue (`self.GetComponentByClass` InActor "/Game/Blueprint/Core/Interactables/Components/AC_BaseInfo.AC_BaseInfo_C"))
  ;[1 0 0] UpdateHUD Selected Object
  (if (`KismetSystemLibrary.IsValid` _returnvalue)
    (`/Game/Blueprint/Core/Gameflow/Playercontrollers/PC_Rts.UpdateSelectedInfo` (`self.GetPCRef`) (`/Game/Blueprint/Core/Interactables/Components/AC_BaseInfo.BaseInfo` _returnvalue) (`/Game/Blueprint/Core/Interactables/Components/AC_BaseInfo.classTag` _returnvalue))
    (`/Game/Blueprint/Core/Gameflow/Playercontrollers/PC_Rts.UseRallyPoint` (`self.GetPCRef`) (`/Game/Blueprint/Core/Interactables/Components/AC_BaseInfo.RallyPoint` _returnvalue))))

(event `DeselectOnServer`
  ;[0.875 0 0.008648] Deselect on Server
  (if (!= (`self.LastSelectedActor`) null)
    (`self.Change Decal Effect` (`self.LastSelectedActor`) (struct) true)
    (`self.DeselectOnClients` (`self.LastSelectedActor`))))

(event `AddDecalOnServer`
  (params (Actor :type "Actor Object Reference"))
  ;[1 0 0.009947] GetColor And Change Decal on Server
  (set `self.LastSelectedActor` Actor)
  (bind (_name _color) (`/Game/Blueprint/Core/Gameflow/Playercontrollers/PC_Rts.GetPlayerInfo` (`self.GetPCRef`) (`/Game/Blueprint/Core/Gameflow/Playercontrollers/PC_Rts.GetPlayerIndex` (`self.GetPCRef`))))
  (`self.Change Decal Effect` Actor _color)
  (`self.ReplicateDecalMulticast` Actor _color))

(event `DeselectOnClients`
  (params (Actor :type "Actor Object Reference"))
  ;[1 0 0.5405] Deselect Multicast
  (`self.Change Decal Effect` Actor (struct) true))

(event `ReplicateDecalMulticast`
  (params (InActor :type "Actor Object Reference") (InColor :type "Color Structure"))
  ;[1 0 0.9789] Multicast Color Decal
  (`self.Change Decal Effect` InActor InColor))

(event `EnhancedInput|/Game/Blueprint/Core/Input/IA_MarkOnMap`
  (params (ActionValue :type "Vector2D Structure") (ElapsedSeconds :type "Float (double-precision)") (TriggeredSeconds :type "Float (double-precision)") (InputAction :type "InputAction Object Reference" :default "/Game/Blueprint/Core/Input/IA_MarkOnMap.IA_MarkOnMap"))
  (bind (_worldlocation _worlddirection) (`PlayerController.DeprojectMousePositionToWorld` (`self.GetPCRef`)))
  ;[0 0.1579 1] MarkUp
  (:`Started`
    (bind (_outhit _returnvalue) (`KismetSystemLibrary.LineTraceSingle` :`Start` _worldlocation :`End` (+ _worldlocation (* _worlddirection 10000.0)) :`TraceChannel` "TraceTypeQuery1" :`DrawTime` 1.0))
    (if _returnvalue
      (`/Game/Blueprint/Core/Gameflow/Playercontrollers/PC_Rts.LoadMarkUp` (`self.GetPCRef`) (`.Location` (`GameplayStatics.BreakHitResult` _outhit)))))
  (:`Completed`
    (`/Game/Blueprint/Core/Gameflow/Playercontrollers/PC_Rts.FocusMarkUI` (`self.GetPCRef`))))

(event `GetPlayerInfo`
  (params (Start :type "Vector Structure"))
  (bind _pcref (`self.GetPCRef`))
  ;[1 0.009549 0] FeedBackCursor-NOT IN USE
  (bind (_name _color) (`/Game/Blueprint/Core/Gameflow/Playercontrollers/PC_Rts.GetPlayerInfo` _pcref (`/Game/Blueprint/Core/Gameflow/Playercontrollers/PC_Rts.GetPlayerIndex` _pcref)))
  (`|SpawnActorFromClass` "/Game/Blueprint/Core/Interactables/ActorCursor/BP_FeedbackCursor.BP_FeedbackCursor_C" (`KismetMathLibrary.MakeTransform` Start) "Undefined" "MultiplyWithRoot" null _name _color null))

(event `SpawnMiddleClickWidget`
  (params (Selection :type "/Game/Blueprint/Core/Interactables/Data/enums/EMarkSelection Enum" :default "NewEnumerator0") (SpawnPosition :type "Vector Structure"))
  ;[0.9688 0 0.02332] MiddleClickWidget
  (`/Game/Blueprint/Core/Gameflow/Playercontrollers/PC_Rts.SpawnMarkActor` (`self.GetPCRef`) Selection SpawnPosition))

(event `EnhancedInput|/Game/Blueprint/Core/Input/IA_ZoomOut`
  (params (ActionValue :type "Float (double-precision)") (ElapsedSeconds :type "Float (double-precision)") (TriggeredSeconds :type "Float (double-precision)") (InputAction :type "InputAction Object Reference" :default "/Game/Blueprint/Core/Input/IA_ZoomOut.IA_ZoomOut"))
  ;[0 0.08737 1] Zoom
  (:`Triggered`
    (bind (_direction _output) (`Timeline|ZoomMove` :!label _label)
      (:`Update`
        (`self.SetCameraPosition` (`self.Camera`) _output "/Game/Blueprint/Core/Interactables/Data/curves/C_CameraPos.C_CameraPos")
        (`self.Set Camera Angle` (`self.Camera`) "/Game/Blueprint/Core/Interactables/Data/curves/C_CameraPos.C_CameraPos" _output)))))

(event `EnhancedInput|/Game/Blueprint/Core/Input/IA_ZoomIn`
  (params (ActionValue :type "Float (double-precision)") (ElapsedSeconds :type "Float (double-precision)") (TriggeredSeconds :type "Float (double-precision)") (InputAction :type "InputAction Object Reference" :default "/Game/Blueprint/Core/Input/IA_ZoomIn.IA_ZoomIn"))
  ;[0 0.08737 1] Zoom
  (:`Triggered`
    (goto _label :!via `Reverse`)))

(event `EnhancedInput|/Game/Blueprint/Core/Input/IA_Right`
  (params (ActionValue :type "Vector2D Structure") (ElapsedSeconds :type "Float (double-precision)") (TriggeredSeconds :type "Float (double-precision)") (InputAction :type "InputAction Object Reference" :default "/Game/Blueprint/Core/Input/IA_Right.IA_Right"))
  (bind (_outhit _returnvalue) (`self.GetMousePosition` "TraceTypeQuery5"))
  (bind _lastselectedactor (`self.LastSelectedActor`))
  (bind (_deltax _deltay) (`PlayerController.GetInputMouseDelta` (`self.GetPCRef`)))
  (bind (_bblockinghit _binitialoverlap _time _distance _location _impactpoint _normal _impactnormal _physmat _hitactor) (`GameplayStatics.BreakHitResult` _outhit))
  (bind _returnvalue_2 (`self.GetComponentByClass` _lastselectedactor "/Game/Blueprint/Core/Interactables/Components/AC_UnitInfo.AC_UnitInfo_C"))
  (bind (_x _y) (`KismetMathLibrary.BreakVector2D` (* (`KismetMathLibrary.MakeVector2D` _deltay _deltax) (* (`self.SpeedCamera`) -1.0))))
  ;[0 0.171 1] GrabHand
  (:`Triggered`
    (`PawnMovementComponent.AddInputVector` (`self.FloatingPawnMovement`) (`KismetMathLibrary.MakeVector` _x _y) false)
    (`/Game/Blueprint/Core/Gameflow/Playercontrollers/PC_Rts.CursorChange` (`self.GetPCRef`) true)
    (if (`KismetSystemLibrary.IsValid` _lastselectedactor)
      (if (`KismetSystemLibrary.IsValid` _returnvalue_2)
        (if _returnvalue
          (if _bblockinghit
            (if (`KismetSystemLibrary.IsValid` _hitactor)
              (`/Game/Blueprint/Core/Actions/BPI_Orders.GiveOrderToLocation` _returnvalue_2 (struct :`TagName` "Actions.Units.Follow") _location)
              (if (`KismetSystemLibrary.IsValid` (`self.GetComponentByClass` _hitactor "/Game/Blueprint/Core/Interactables/Components/AC_ResourceInfo.AC_ResourceInfo_C"))
                (`/Game/Blueprint/Core/Interactables/BaseActorsRTS/BaseUnit.BindOverlapGather` (`self.GetBaseUnitRef` (`self.LastSelectedActor`)))
                (elif (`KismetSystemLibrary.IsValid` (`self.GetComponentByClass` _hitactor "/Game/Blueprint/Core/Interactables/Components/AC_BuildingInfo.AC_BuildingInfo_C"))
                  (`/Game/Blueprint/Core/Interactables/BaseActorsRTS/BaseUnit.BindOverlapConstruction` (`self.GetBaseUnitRef` (`self.LastSelectedActor`)) _location)))))))))
  (:`Completed`
    (`/Game/Blueprint/Core/Gameflow/Playercontrollers/PC_Rts.CursorChange` (`self.GetPCRef`) false)))

(fn `Change Decal Effect`
  (params (InActor :type "Actor Object Reference") (Color :type "Color Structure") (Hidden :type Boolean))
  (bind _returnvalue (`self.GetComponentByClass` InActor "/Script/Engine.DecalComponent"))
  (if (!= _returnvalue null)
    (`SceneComponent.SetHiddenInGame` _returnvalue (`local.Hidden`) false)
    (`DecalComponent.SetDecalColor` _returnvalue (`KismetMathLibrary.Conv_ColorToLinearColor` (`local.Color`)))))

(fn `GetAIRef`
  (params (Object :type "Actor Object Reference"))
  (returns (AIRef :type "/Game/Blueprint/Core/AI/AI_BaseUnit Object Reference"))
  (`self.AIRef`
    (:`then`
      (return (`self.AIRef`)))
    (:`else`
      (bind _asai_base_unit (cast `/Game/Blueprint/Core/AI/AI_BaseUnit` (`AIBlueprintHelperLibrary.GetAIController` Object))
        (:`then`
          (set `self.AIRef` _asai_base_unit)
          (return (`self.AIRef`)))
        (:`CastFailed`
          (`KismetSystemLibrary.PrintString` "AIBaseUnit Ref Failed"))))))

(fn `GetBaseUnitRef`
  (params (Object :type "Object Object Reference"))
  (returns (BaseUnitRef :type "/Game/Blueprint/Core/Interactables/BaseActorsRTS/BaseUnit Object Reference"))
  (bind _asbase_unit (cast `/Game/Blueprint/Core/Interactables/BaseActorsRTS/BaseUnit` Object))
  (return _asbase_unit))

(fn `GetBPAWorkerRef`
  (params (Mesh :type "SkeletalMeshComponent Object Reference"))
  (returns (BPAWorkerRef :type "/Game/Assets/AssetPack/Toon_RTS_Elves/Animations/Worker/BPA_Worker Object Reference"))
  (`self.BPAWorkerRef`
    (:`then`
      _)
    (:`else`
      (bind _asbpa_worker (cast `/Game/Assets/AssetPack/Toon_RTS_Elves/Animations/Worker/BPA_Worker` (`SkeletalMeshComponent.GetAnimInstance` Mesh)))
      (set `self.BPAWorkerRef` _asbpa_worker)))
  (return (`self.BPAWorkerRef`)))

(fn `GetGSRef`
  (returns (GSRef :type "/Game/Blueprint/Core/Gameflow/GameStates/GS_Rts Object Reference"))
  (`self.GSRef`
    (:`then`
      _)
    (:`else`
      (bind _asgs_rts (cast `/Game/Blueprint/Core/Gameflow/GameStates/GS_Rts` (`GameplayStatics.GetGameState`)))
      (set `self.GSRef` _asgs_rts)))
  (return (`self.GSRef`)))

(fn `GetMousePosition`
  (params (TraceChannel :type "ETraceTypeQuery Enum" :default "TraceTypeQuery1"))
  (returns (OutHit :type "HitResult Structure") (ReturnValue :type Boolean))
  (locals (NewLocalVar :type "Array of EObjectTypeQuery Enum"))
  (bind (_worldlocation _worlddirection) (`PlayerController.DeprojectMousePositionToWorld` (`self.GetPCRef`)))
  (bind (_outhit _returnvalue) (`KismetSystemLibrary.LineTraceSingle` :`Start` _worldlocation :`End` (+ _worldlocation (* _worlddirection 100000.0)) :`TraceChannel` TraceChannel :`DrawTime` 2.0))
  (return _outhit _returnvalue))

(fn `GetPCRef`
  (returns (PCRef :type "/Game/Blueprint/Core/Gameflow/Playercontrollers/PC_Rts Object Reference"))
  (`self.PCRef`
    (:`then`
      _)
    (:`else`
      (bind _aspc_rts (cast `/Game/Blueprint/Core/Gameflow/Playercontrollers/PC_Rts` (`self.GetOwner`)))
      (set `self.PCRef` _aspc_rts)))
  (return (`self.PCRef`)))

(fn `GetPSRef`
  (returns (PSRef :type "/Game/Blueprint/Core/Gameflow/PlayerStates/PS_Rts Object Reference"))
  (`self.PSRef`
    (:`then`
      _)
    (:`else`
      (bind _asps_rts (cast `/Game/Blueprint/Core/Gameflow/PlayerStates/PS_Rts` (`self.PlayerState`)))
      (set `self.PSRef` _asps_rts)))
  (return (`self.PSRef`)))

(fn `Set Camera Angle`
  (params (InCamera :type "SceneComponent Object Reference") (Curve :type "CurveVector Object Reference") (InValue :type "Float (double-precision)"))
  (bind _incamera (`local.InCamera`))
  (`SceneComponent.K2_SetWorldRotation` _incamera (`KismetMathLibrary.MakeRotator` (.roll (`SceneComponent.RelativeRotation` _incamera)) (`KismetMathLibrary.Lerp` (.y (`CurveVector.GetVectorValue` Curve 1.0)) (.y (`CurveVector.GetVectorValue` Curve 0.0)) InValue) (.yaw (`SceneComponent.RelativeRotation` _incamera))) false false))

(fn `SetCameraPosition`
  (params (InCamera :type "SceneComponent Object Reference") (InValue :type "Float (double-precision)") (InCurve :type "CurveVector Object Reference"))
  (locals (ZValue :type "Float (double-precision)" :default 0.0))
  (bind _incamera (`local.InCamera`))
  (`SceneComponent.K2_SetWorldLocation` _incamera (`KismetMathLibrary.MakeVector` (.x (`SceneComponent.K2_GetComponentLocation` _incamera)) (.y (`SceneComponent.K2_GetComponentLocation` _incamera)) (`KismetMathLibrary.Lerp` (.z (`CurveVector.GetVectorValue` InCurve 0.0)) (.z (`CurveVector.GetVectorValue` InCurve 1.0)) InValue)) false false))

(fn `SphereTraceWithMouse`
  (params (TraceChannel :type "ETraceTypeQuery Enum" :default "TraceTypeQuery1") (Radius :type "Float (single-precision)") (ObjectTypes :type "Array of EObjectTypeQuery Enum (by ref)"))
  (returns (ReturnValue :type Boolean) (HitActor :type "Actor Object Reference") (ActorLocation :type "Vector Structure"))
  (locals (NewLocalVar_0 :type "Array of Actor Object Reference"))
  (bind (_outhit _returnvalue) (`self.GetMousePosition` TraceChannel))
  (bind (_bblockinghit _binitialoverlap _time _distance _location) (`GameplayStatics.BreakHitResult` _outhit))
  (if _returnvalue
    (if _bblockinghit
      (bind _outactors (`KismetSystemLibrary.SphereOverlapActors` _location Radius ObjectTypes))
      (for _array_element _outactors
        (if (`KismetSystemLibrary.IsValid` (`self.GetComponentByClass` _array_element "/Game/Blueprint/Core/Interactables/Components/AC_ResourceInfo.AC_ResourceInfo_C"))
          (return true _array_element (`self.K2_GetActorLocation` _array_element))))
      (return false null (0.0 0.0 0.0)))))

(fn `UserConstructionScript`)