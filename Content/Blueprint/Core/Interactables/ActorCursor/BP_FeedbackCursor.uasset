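; BP_FeedbackCursor is a short-lived cursor feedback actor that marks a player with their name and team color.
; On BeginPlay it sets a one-second lifespan, writes the player name into a text render component and tints it with the team color.
; It also passes the team color to a Niagara effect's ColorArrow parameter, coloring the effect to match.
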(event `self.ReceiveBeginPlay`
  (bind _playername (`self.PlayerName`))
  (`self.SetLifeSpan` 1.0)
  (`TextRenderComponent.K2_SetText` _playername (`KismetTextLibrary.Conv_NameToText` (`self.Name`)))
  (`TextRenderComponent.SetTextRenderColor` _playername (`self.TeamColor`))
  (`NiagaraComponent.SetVariableLinearColor` (`self.Niagara`) "ColorArrow" (`KismetMathLibrary.Conv_ColorToLinearColor` (`self.TeamColor`))))

(fn `UserConstructionScript`)