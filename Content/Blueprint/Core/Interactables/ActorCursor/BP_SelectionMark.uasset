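; BP_SelectionMark is a temporary RTS cursor marker actor that signals a Warning or Attack selection.
; On BeginPlay it sets its lifespan and gives its W_SelectableCursor widget the texture matching the selection type.
; Tick tints the decal with the player color and pulses actor scale along a curve on a two-second loop.
; When destroyed, it clears SelectionActor on the cached PC_Rts player controller.
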(event `self.ReceiveBeginPlay`
  (bind _image (`/Game/Blueprint/Core/Widgets/W_SelectableCursor.Image` (`self.SelectableCursor`)))
  (bind _asw_selectable_cursor (cast `/Game/Blueprint/Core/Widgets/W_SelectableCursor` (`WidgetComponent.GetWidget` (`self.Widget`))))
  (set `self.SelectableCursor` _asw_selectable_cursor)
  (set `self.InitScale` (`self.GetActorScale3D`))
  (`self.SetLifeSpan` (`self.In Lifespan`))
  (bind _values (`BlueprintMapLibrary.Map_Values` (`self.Textures`)))
  (switch `/Game/Blueprint/Core/Interactables/Data/enums/EMarkSelection` (`self.Selection`)
    (:`NewEnumerator1`
      (`Image.SetBrushFromSoftTexture` _image (`|GetArrayItem` _values) false))
    (:`NewEnumerator2`
      (`Image.SetBrushFromSoftTexture` _image (`|GetArrayItem` _values 1) false))))

(event `self.ReceiveTick`
  (params (DeltaSeconds :type "Float (single-precision)"))
  (`DecalComponent.SetDecalColor` (`self.Decal`) (`KismetMathLibrary.Conv_ColorToLinearColor` (`self.PlayerColor`)))
  (bind _output_get (set `self.Delta` (+ DeltaSeconds (`self.Delta`))))
  (`self.SetActorScale3D` (+ (* (`self.InitScale`) (`CurveFloat.GetFloatValue` (`self.CurveMove`) _output_get)) 0.5))
  (if (> (`self.Delta`) 2.0)
    (set `self.Delta` 0.0)))

(event `self.ReceiveDestroyed`
  (set `/Game/Blueprint/Core/Gameflow/Playercontrollers/PC_Rts.SelectionActor` null (`self.GetPCRef`)))

(fn `DestroyAfterTime`
  (`self.SetLifeSpan` 0.0))

(fn `GetPCRef`
  (returns (PCRef :type "/Game/Blueprint/Core/Gameflow/Playercontrollers/PC_Rts Object Reference"))
  (`self.PCRef`
    (:`then`
      _)
    (:`else`
      (bind _aspc_rts (cast `/Game/Blueprint/Core/Gameflow/Playercontrollers/PC_Rts` (`GameplayStatics.GetPlayerController` 0)))
      (set `self.PCRef` _aspc_rts)))
  (return (`self.PCRef`)))

(fn `SetScale`
  (params (Scale :type "Float (single-precision)") (InDecal :type "DecalComponent Object Reference"))
  (`DecalFunctions.SetDecalSize` InDecal (* (`self.InitScale`) Scale)))

(fn `UserConstructionScript`)