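; BP_GASCharacter is a character Blueprint among the base RTS actors that configures its appearance from unit data.
; On BeginPlay it passes its ClassTag to the ACUnitInfo component and loads the matching info as an instanced struct.
; If that struct is valid, ACUnitInfo applies its skeletal mesh to the Mesh component and its scale to the Decal component.
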(event `self.ReceiveBeginPlay`
  (set `/Game/Blueprint/Core/Interactables/Components/AC_BaseInfo.classTag` (`self.classTag`) (`self.AC_UnitInfo`))
  (bind _outinfo (`/Game/Blueprint/Core/Interactables/Components/AC_UnitInfo.Load Info` (`self.AC_UnitInfo`) (`self.classTag`)))
  (bind _value (`StructUtilsFunctionLibrary.GetInstancedStructValue` _outinfo)
    (:`Valid`
      (bind ((`Mesh_32_48E71EB2408CDDB936947EA07A6A50EB` _mesh) (`DecalScale_37_4E2C1B84465FE4AEE4E0CA999320E4AB` _decalscale)) (break `/Game/Blueprint/Core/Interactables/Data/structures/ST_Units` _value))
      (`/Game/Blueprint/Core/Interactables/Components/AC_BaseInfo.LoadSkeletalMesh` (`self.AC_UnitInfo`) (`self.Mesh`) _mesh)
      (`/Game/Blueprint/Core/Interactables/Components/AC_BaseInfo.LoadDecalSize` (`self.AC_UnitInfo`) (`self.Decal`) self _decalscale))))

(fn `UserConstructionScript`)