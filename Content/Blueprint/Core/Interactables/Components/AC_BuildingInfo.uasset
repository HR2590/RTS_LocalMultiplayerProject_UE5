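; Building info component that holds a building's data as an instanced struct and tracks its construction progress.
; LoadInfo fills the struct from the DT_Buildings row matching a class tag, while SetInfo assigns it directly.
; BuildingUp adds to the construction percent and, at completion, loads the building mesh and scale onto the BaseBuilding owner and clears the under-construction flag, then stores the updated struct.
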(event `BuildingUp`
  (params (Value :type "Float (double-precision)"))
  (bind _structout (setmembers `/Game/Blueprint/Core/Interactables/Data/structures/ST_Buildings` :`StructRef` (`self.Data`)))
  (bind ((`Mesh_35_797926D04D581ED3CFFBC7AF6F5DC608` _mesh) (`StaticMeshScale_41_C175D43842C99A6DEFE7EBAEA27B9F95` _staticmeshscale) (`UnderConstruction_65_958C5E55490939DAD387A98EC5C5380E` _underconstruction) (`UndeConstructionPercent_70_058B2806422616B30519BB9CB4FFF32F` _undeconstructionpercent)) (break `/Game/Blueprint/Core/Interactables/Data/structures/ST_Buildings` _structout))
  (`|VariableSetRef` _undeconstructionpercent (+ Value _undeconstructionpercent))
  (if (>= _undeconstructionpercent 1.0)
    (bind _asbase_building (cast `/Game/Blueprint/Core/Interactables/BaseActorsRTS/BaseBuilding` (`self.GetOwner`)))
    (`self.LoadMesh` (`/Game/Blueprint/Core/Interactables/BaseActorsRTS/BaseBuilding.Mesh` _asbase_building) _mesh _staticmeshscale)
    (`|VariableSetRef` _underconstruction))
  (bind _returnvalue (`StructUtilsFunctionLibrary.MakeInstancedStruct` _structout))
  (set `self.BaseInfo` _returnvalue))

(fn `LoadInfo`
  (params (classTag :type "GameplayTag Structure"))
  (returns (OutInfo :type "InstancedStruct Structure"))
  (bind _returnvalue (`self.LoadTag` classTag))
  (bind _returnvalue_2 (`|GetDataTableRow` "/Game/Blueprint/Core/Interactables/Data/datatables/DT_Buildings.DT_Buildings" _returnvalue)
    (:`then`
      (bind _returnvalue_3 (`StructUtilsFunctionLibrary.MakeInstancedStruct` _returnvalue_2))
      (bind _output_get (set `self.BaseInfo` _returnvalue_3))
      (return _output_get))))

(fn `SetInfo`
  (params (BaseInfo :type "InstancedStruct Structure"))
  (set `self.BaseInfo` BaseInfo)
  (return))