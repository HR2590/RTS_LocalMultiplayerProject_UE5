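; AC_UnitInfo is a component that holds a unit's base data and relays orders to the unit's AI.
; Order events (plain, location, actor, location with ID) pass through Server-named events, which call the matching functions on the AI reference.
; LoadInfo looks up a DT_Units row by class tag and stores it as an instanced struct in BaseInfo.
; The GiveOrderServer function is an empty stub.
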(event `GiveOrderLocationClient`
  (params (InOrder :type "GameplayTag Structure") (Location :type "Vector Structure"))
  (`self.GiveOrdertoLocationServer` InOrder Location))

(event `GiveOrderClient`
  (params (InOrder :type "GameplayTag Structure"))
  (`self.GiveOrderServe` InOrder))

(event `/Game/Blueprint/Core/Actions/BPI_Orders.GiveOrder`
  (params (InOrder :type "GameplayTag Structure"))
  (`self.GiveOrderServe` InOrder))

(event `GiveOrderServe`
  (params (InOrder :type "GameplayTag Structure"))
  (`/Game/Blueprint/Core/Actions/BPI_Orders.GiveOrder` (`self.GetAIRef`) InOrder))

(event `GiveOrdertoLocationServer`
  (params (Order :type "GameplayTag Structure") (Location :type "Vector Structure"))
  (`/Game/Blueprint/Core/Actions/BPI_Orders.GiveOrderToLocation` (`self.GetAIRef`) Order Location))

(event `/Game/Blueprint/Core/Actions/BPI_Orders.GiveOrderToLocation`
  (params (InOrder :type "GameplayTag Structure") (Location :type "Vector Structure"))
  (`self.GiveOrdertoLocationServer` InOrder Location))

(event `GiveOrderActorServer`
  (params (Order :type "GameplayTag Structure"))
  (`/Game/Blueprint/Core/Actions/BPI_Orders.GiveOrderToActor` (`self.GetAIRef`) Order))

(event `/Game/Blueprint/Core/Actions/BPI_Orders.GiveOrderToActor`
  (params (InOrder :type "GameplayTag Structure"))
  (`self.GiveOrderActorServer` InOrder))

(event `GiveOrderToLocationWithIDServer`
  (params (Order :type "GameplayTag Structure") (Location :type "Vector Structure"))
  (`/Game/Blueprint/Core/Actions/BPI_Orders.GiveOrderToLocationWithID` (`self.GetAIRef`) Order Location))

(event `/Game/Blueprint/Core/Actions/BPI_Orders.GiveOrderToLocationWithID`
  (params (InOrder :type "GameplayTag Structure") (Location :type "Vector Structure"))
  (`self.GiveOrderToLocationWithIDServer` InOrder Location))

(fn `GiveOrderServer`
  (params (InOrder1 :type "GameplayTag Structure")))

(fn `Load Info`
  (params (classTag :type "GameplayTag Structure"))
  (returns (OutInfo :type "InstancedStruct Structure"))
  (bind _returnvalue (`self.LoadTag` classTag))
  (bind _returnvalue_2 (`|GetDataTableRow` "/Game/Blueprint/Core/Interactables/Data/datatables/DT_Units.DT_Units" _returnvalue)
    (:`then`
      (bind _returnvalue_3 (`StructUtilsFunctionLibrary.MakeInstancedStruct` _returnvalue_2))
      (bind _output_get (set `self.BaseInfo` _returnvalue_3))
      (return _output_get))))