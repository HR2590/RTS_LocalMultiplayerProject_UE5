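; AC_BaseInfo is an interactables component of shared helpers for setting up an actor's visuals and accessing its class tag and AI controller.
; It blocking-loads static and skeletal meshes onto given components, scaling static ones, and sizes decals from the actor's larger horizontal extent.
; LoadTag returns a valid tag's name if it matches ClassContainer.
; GetAIRef lazily caches the owner's AI_BaseUnit controller, printing on cast failure.
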(fn `GetAIRef`
  (returns (AIController :type "/Game/Blueprint/Core/AI/AI_BaseUnit Object Reference"))
  (`self.AIController`
    (:`then`
      (return (`self.AIController`)))
    (:`else`
      (bind _asai_base_unit (cast `/Game/Blueprint/Core/AI/AI_BaseUnit` (`AIBlueprintHelperLibrary.GetAIController` (`self.GetOwner`)))
        (:`then`
          (set `self.AIController` _asai_base_unit)
          (return (`self.AIController`)))
        (:`CastFailed`
          (`KismetSystemLibrary.PrintString` "AIRef failed cast"))))))

(fn `LoadDecalSize`
  (params (DecalComponent :type "DecalComponent Object Reference") (Actor :type "Actor Object Reference") (DecalScale :type "Float (double-precision)"))
  (bind _returnvalue (* (`KismetMathLibrary.FMax` (.x (`.BoxExtent` (`Actor.GetActorBounds` Actor false false))) (.y (`.BoxExtent` (`Actor.GetActorBounds` Actor false false)))) DecalScale))
  (`DecalFunctions.SetDecalSize` DecalComponent (`KismetMathLibrary.MakeVector` (.x (`DecalComponent.DecalSize` DecalComponent)) _returnvalue _returnvalue)))

(fn `LoadMesh`
  (params (StaticMeshComponent :type "StaticMeshComponent Object Reference") (Mesh :type "StaticMesh Soft Object Reference") (Scale :type "Float (double-precision)"))
  (bind _returnvalue (`KismetSystemLibrary.LoadAsset_Blocking` Mesh))
  (bind _asstatic_mesh (cast `StaticMesh` _returnvalue))
  (`StaticMeshComponent.SetStaticMesh` StaticMeshComponent _asstatic_mesh)
  (`SceneComponent.SetWorldScale3D` StaticMeshComponent (* (`SceneComponent.K2_GetComponentScale` StaticMeshComponent) Scale)))

(fn `LoadSkeletalMesh`
  (params (SkeletalMesh :type "SkeletalMeshComponent Object Reference") (Asset :type "Object Soft Object Reference"))
  (bind _returnvalue (`KismetSystemLibrary.LoadAsset_Blocking` Asset))
  (bind _asskeletal_mesh (cast `SkeletalMesh` _returnvalue))
  (`SkeletalMeshComponent.SetSkeletalMeshAsset` SkeletalMesh _asskeletal_mesh))

(fn `LoadTag`
  (params (classTag :type "GameplayTag Structure"))
  (returns (ReturnValue :type Name))
  (locals (ClassName :type Name))
  (if (`BlueprintGameplayTagLibrary.IsGameplayTagValid` classTag)
    (if (`BlueprintGameplayTagLibrary.MatchesAnyTags` (`local.classTag`) (`self.ClassContainer`))
      (return (`BlueprintGameplayTagLibrary.GetTagName` (`local.classTag`))))))