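; Resource info component for interactable resources, tracking a depletable value that refills after a timed reset.
; LoadInfo uses a class tag to pull a DT_Resources row into BaseInfo as an instanced struct.
; DecrementResource clamps the value and, on depletion, synchronously loads the destroyed mesh onto the owning BaseResource and starts the reset timer.
; Reset restores the maximum value, reinitializes the mesh, updates BaseInfo and clears the timer.
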(event `DecrementResource`
  (params (Value :type Integer))
  (bind _structout (setmembers `/Game/Blueprint/Core/Interactables/Data/structures/ST_Resources` :`StructRef` (`self.Info`)))
  (bind ((`currentvalue_23_F327E2DC412AE39E27D3E585BE5A9C31` _currentvalue) (`maxvalue_25_1189AFAE493C947529E96AA4C89AE723` _maxvalue)) (break `/Game/Blueprint/Core/Interactables/Data/structures/ST_Resources` _structout))
  (bind _returnvalue (`KismetMathLibrary.Clamp` (- _currentvalue Value) 0 _maxvalue))
  (`|VariableSetRef` _currentvalue _returnvalue)
  (bind _returnvalue_2 (`StructUtilsFunctionLibrary.MakeInstancedStruct` (`self.Info`)))
  (set `self.BaseInfo` _returnvalue_2)
  (if (<= _returnvalue 0)
    (if (not (`KismetSystemLibrary.K2_IsTimerActiveHandle` (`self.ResetTimer`)))
      (`self.LoadDestroyedMesh`)
      (bind _returnvalue_3 (`KismetSystemLibrary.K2_SetTimerDelegate` (delegate `Reset`) (`.ResetTime_38_C89B0394499F3F97AFEB258C5BAD073F` (break `/Game/Blueprint/Core/Interactables/Data/structures/ST_Resources` (`self.Info`)))))
      (set `self.ResetTimer` _returnvalue_3))))

(event `Reset`
  (bind _structout (setmembers `/Game/Blueprint/Core/Interactables/Data/structures/ST_Resources` :`StructRef` (`self.Info`)))
  (bind ((`currentvalue_23_F327E2DC412AE39E27D3E585BE5A9C31` _currentvalue) (`maxvalue_25_1189AFAE493C947529E96AA4C89AE723` _maxvalue)) (break `/Game/Blueprint/Core/Interactables/Data/structures/ST_Resources` _structout))
  (`|VariableSetRef` _currentvalue _maxvalue)
  (`self.InitilizeMesh`)
  (bind _returnvalue (`StructUtilsFunctionLibrary.MakeInstancedStruct` _structout))
  (set `self.BaseInfo` _returnvalue)
  (`KismetSystemLibrary.K2_ClearAndInvalidateTimerHandle` (`self.ResetTimer`)))

(fn `LoadDestroyedMesh`
  (bind _asbase_resource (cast `/Game/Blueprint/Core/Interactables/BaseActorsRTS/BaseResource` (`self.GetOwner`)))
  (bind _returnvalue (`KismetSystemLibrary.LoadAsset_Blocking` (`.DestroyedMesh_41_A766CD5043D13D7F32490095EFA6BE8F` (break `/Game/Blueprint/Core/Interactables/Data/structures/ST_Resources` (`self.Info`)))))
  (bind _asstatic_mesh (cast `StaticMesh` _returnvalue))
  (`StaticMeshComponent.SetStaticMesh` (`/Game/Blueprint/Core/Interactables/BaseActorsRTS/BaseResource.Mesh` _asbase_resource) _asstatic_mesh))

(fn `LoadInfo`
  (params (classTag :type "GameplayTag Structure"))
  (returns (OutInfo :type "InstancedStruct Structure"))
  (bind _returnvalue (`self.LoadTag` classTag))
  (bind _returnvalue_2 (`|GetDataTableRow` "/Game/Blueprint/Core/Interactables/Data/datatables/DT_Resources.DT_Resources" _returnvalue)
    (:`then`
      (bind _returnvalue_3 (`StructUtilsFunctionLibrary.MakeInstancedStruct` _returnvalue_2))
      (bind _output_get (set `self.BaseInfo` _returnvalue_3))
      (return _output_get))))